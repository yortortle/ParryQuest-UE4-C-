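; Early-stage 2D NPC Blueprint with a flipbook sprite; at runtime it only prints a debug "Hello" on BeginPlay.
; FLIP fires EVENTSET when velocity is non-zero to set the flipbook, with no asset specified, but nothing here calls FLIP.
; Tick is empty, and leftover timer, movement input, DUPLOG flipbook and IsMovingRight direction nodes are disconnected.
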(event Custom|EVENTSET
  (Sprite|SetFlipbook (Variables|Default|GetSprite)))

(event EventTick
  (params (DeltaSeconds :type Float%20%28single-precision%29)))

(event EventBeginPlay
  (Development|PrintString "Hello"))

(fn ConstructionScript)

(fn FLIP
  (if (> (Math|Vector|VectorLength (Transformation|GetVelocity)) 0.0)
    (CallFunction|EVENTSET)))