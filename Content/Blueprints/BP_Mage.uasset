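; BP_Mage is a talking NPC that shows a dialogue widget when a BP_SwordMan overlaps its capsule.
; Any overlap pauses WalkTimer, though this graph never sets that timer; only a swordsman is stored as CurrentNPC and triggers dialogue.
; ShowDialogue creates BP_Dialogue with the mage as NPC, then advances DialogueIndex, wrapping at the end.
; When the stored swordsman leaves, the widget is removed and the timer unpauses.
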(event OnComponentBeginOverlap(CapsuleComponent)
  (params (OverlappedComponent :type Primitive%20Component%20Object%20Reference) (OtherActor :type Actor%20Object%20Reference) (OtherComp :type Primitive%20Component%20Object%20Reference) (OtherBodyIndex :type Integer) (bFromSweep :type Boolean) (SweepResult :type Hit%20Result%20Structure%20%28by%20ref%29))
  (Utilities|Time|PauseTimerbyHandle (Variables|Default|GetWalkTimer))
  (bind _asbp_sword_man (Utilities|Casting|CastToBP_SwordMan OtherActor))
  (Variables|Default|SetCurrentNPC _asbp_sword_man)
  (CallFunction|ShowDialogue))

(event OnComponentEndOverlap(CapsuleComponent)
  (params (OverlappedComponent :type Primitive%20Component%20Object%20Reference) (OtherActor :type Actor%20Object%20Reference) (OtherComp :type Primitive%20Component%20Object%20Reference) (OtherBodyIndex :type Integer))
  (if (== OtherActor (Variables|Default|GetCurrentNPC))
    (CallFunction|HideDialogue)
    (Utilities|Time|UnpauseTimerbyHandle (Variables|Default|GetWalkTimer))))

(fn ConstructionScript)

(fn ShowDialogue
  (bind _returnvalue (UserInterface|CreateWidget "/Game/Blueprints/BP_Dialogue.BP_Dialogue_C" 0 self))
  (bind _output_get (Variables|Default|SetDialogue_Widget _returnvalue))
  (UserInterface|Viewport|AddtoViewport _output_get 0)
  (if (>= (Variables|Default|GetDialogue_Index) (Utilities|Array|LastIndex (Variables|Default|GetDialogue)))
    (Variables|Default|SetDialogue_Index 0)
    (else
      (Variables|Default|SetDialogue_Index (+ (Variables|Default|GetDialogue_Index) 1)))))

(fn HideDialogue
  (Widget|RemovefromParent (Variables|Default|GetDialogue_Widget)))