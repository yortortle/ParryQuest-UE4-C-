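; BP_MageBOss is a mage boss Blueprint carrying NPC dialogue logic that is currently disconnected.
; ShowDialogue creates a BP_Dialogue widget with itself as NPC and adds it to the viewport; HideDialogue removes it.
; Unreached chains would pause WalkTimer and show dialogue for an overlapping BP_SwordMan, then reverse this when it leaves.
; Both capsule overlap events are empty, so nothing in this Blueprint triggers dialogue.
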(event OnComponentBeginOverlap(CapsuleComponent)
  (params (OverlappedComponent :type Primitive%20Component%20Object%20Reference) (OtherActor :type Actor%20Object%20Reference) (OtherComp :type Primitive%20Component%20Object%20Reference) (OtherBodyIndex :type Integer) (bFromSweep :type Boolean) (SweepResult :type Hit%20Result%20Structure%20%28by%20ref%29)))

(event OnComponentEndOverlap(CapsuleComponent)
  (params (OverlappedComponent :type Primitive%20Component%20Object%20Reference) (OtherActor :type Actor%20Object%20Reference) (OtherComp :type Primitive%20Component%20Object%20Reference) (OtherBodyIndex :type Integer)))

(fn ConstructionScript)

(fn ShowDialogue
  (bind _returnvalue (UserInterface|CreateWidget "/Game/Blueprints/BP_Dialogue.BP_Dialogue_C" 0 self))
  (bind _output_get (Variables|Default|SetDialogue_Widget _returnvalue))
  (UserInterface|Viewport|AddtoViewport _output_get 0))

(fn HideDialogue
  (Widget|RemovefromParent (Variables|Default|GetDialogue_Widget)))